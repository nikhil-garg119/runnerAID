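; Player-flown physics ship that shoots bullets and drives the spawning of an endless vein tunnel.
; Roll, pitch and yaw inputs apply torque against constant angular damping, while a timer-polled throttle sets the forward speed that velocity eases toward each tick.
; Each tunnel section spawns at the previous one's end, randomly rotated after the first, and the growing section count raises minimum throttle.
; Tick also prints a debug readout of flight stats.
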(event Custom|SpawnVein
  (params (Spawn%20Transform :type Transform))
  ;[1 0.1182 0.5808] Spawning Tunnel Veins
  (bind _returnvalue (Game|SpawnActorfromClass "/Game/Blueprints/Spawner.Spawner_C" Spawn%20Transform "AlwaysSpawn" 0 0))
  (bind _output_get (Variables|Default|SetVeinSection _returnvalue))
  (if (Variables|Default|GetRandomRotate)
    (Math|Integer|IncrementInt (Variables|Default|GetVeinCount)
      (:%20%20
        (Class|Actor|AddActorWorldRotation _output_get (Math|Vector|RotatorfromAxisandAngle (Math|Vector|GetForwardVector (Variables|/Game/Blueprints/Spawner.Spawner_C|Getstart _returnvalue)) (Math|Random|RandomFloatinRange 0.0 1.8e+02)))))
    (else
      (Actor|SetLifeSpan _returnvalue 2e+01)))
  (Development|PrintString (Utilities|String|Append (Utilities|String|ToString(Integer) 0) ": " (Utilities|GetObjectName _returnvalue) ": " (Utilities|String|ToString(Vector) (Transformation|GetWorldLocation (Variables|/Game/Blueprints/Spawner.Spawner_C|Getend _returnvalue)))) true true "(R=0.000000,G=0.000000,B=0.000000,A=1.000000)")
  (Variables|Default|SetNext%20Transform (Math|Transform|MakeTransform (Transformation|GetWorldLocation (Variables|/Game/Blueprints/Spawner.Spawner_C|Getend _returnvalue)) (Transformation|GetWorldRotation (Variables|/Game/Blueprints/Spawner.Spawner_C|Getend _returnvalue))))
  (Variables|Default|SetRandomRotate true)
  (if (< (Variables|Default|GetMinThrottle) 99)
    (Variables|Default|SetMinThrottle (+ 10 (/ (Variables|Default|GetVeinCount) 10)))
    (if (< (Variables|Default|GetThrottle) (Variables|Default|GetMinThrottle))
      (Variables|Default|SetThrottle (Variables|Default|GetMinThrottle)))))

(event Custom|Spawn%20Next
  (CallFunction|SpawnVein (Variables|Default|GetNext%20Transform)))

(event EventBeginPlay
  (bind _self self)
  (Utilities|Time|SetTimerbyFunctionName 0 "ThrottleControl" 0.05 true)
  (EventDispatchers|BindEventtoSpawnNextSection (delegate Custom|Spawn%20Next))
  (CallFunction|SpawnVein (Math|Transform|MakeTransform (Transformation|GetWorldLocation (Variables|Default|GetCollision _self)) (Math|Vector|RotatorfromAxisandAngle (Transformation|GetActorForwardVector _self) 0.0)))
  (Utilities|FlowControl|Delay 2.0)
  (CallFunction|SpawnNext))

(event EventTick
  (params (DeltaSeconds :type Float%20%28single-precision%29))
  (bind _collision (Variables|Default|GetCollision))
  (Variables|Default|SetDelta%20Seconds DeltaSeconds)
  (Class|PrimitiveComponent|AddTorqueinDegrees _collision (/ (Math|Vector|NegateVector (Physics|GetPhysicsAngularVelocityinDegrees (Variables|Default|GetCollision) "None")) 0.5) "None" true)
  (Physics|AddForce _collision (Math|Vector|MakeVector 0.0 0.0 (Variables|Default|GetForce%20Z)) "None" true)
  (CallFunction|CalculateSpeed)
  (Development|PrintString (Utilities|String|Append "Speed : " (Utilities|String|ToString(Float) (Variables|Default|GetSpeed)) " 
Throttle : " (Utilities|String|ToString(Integer) (Variables|Default|GetThrottle)) "%" " 
Distance : " (Utilities|String|ToString(Integer) (Variables|Default|GetVeinCount)) " 
Min Throttle : " (Utilities|String|ToString(Integer) (Variables|Default|GetMinThrottle)) " 
Health : " (Utilities|String|ToString(Integer) (Variables|Default|GetHealth))) true true "(R=1.000000,G=1.000000,B=1.000000,A=1.000000)" (Variables|Default|GetDelta%20Seconds)))

(event Input|ActionEvents|InputActionThrottleUP
  (params (Key :type Key%20Structure :default "None"))
  ;[0.1222 0.6799 1] Throttle Input to Booleans
  (:Pressed
    (Variables|Default|SetThrottleUP true))
  (:Released
    (Variables|Default|SetThrottleUP false)))

(event Input|ActionEvents|InputActionThrottleDOWN
  (params (Key :type Key%20Structure :default "None"))
  ;[0.1222 0.6799 1] Throttle Input to Booleans
  (:Pressed
    (Variables|Default|SetThrottleDOWN true))
  (:Released
    (Variables|Default|SetThrottleDOWN false)))

(event Input|AxisEvents|InputAxisRoll
  (params (AxisValue :type Float%20%28single-precision%29))
  ;[0.1853 0.3411 1] Roll, Pitch & Yaw Input to Torque
  (Variables|Default|SetXAxis AxisValue)
  (Class|PrimitiveComponent|AddTorqueinDegrees (Variables|Default|GetCollision) (Math|Vector|Lerp(Vector) "0, 0, 0" (* (* AxisValue (Variables|Default|GetAirHandling)) (Math|Vector|GetForwardVector (Variables|Default|GetCollision))) 0.1) "None" true))

(event Input|AxisEvents|InputAxisPitch
  (params (AxisValue :type Float%20%28single-precision%29))
  ;[0.1853 0.3411 1] Roll, Pitch & Yaw Input to Torque
  (Variables|Default|SetYAxis AxisValue)
  (Class|PrimitiveComponent|AddTorqueinDegrees (Variables|Default|GetCollision) (Math|Vector|Lerp(Vector) "0, 0, 0" (* (* AxisValue (Variables|Default|GetAirHandling)) (Math|Vector|GetRightVector (Variables|Default|GetCollision))) 0.1) "None" true))

(event Input|AxisEvents|InputAxisYaw
  (params (AxisValue :type Float%20%28single-precision%29))
  ;[0.1853 0.3411 1] Roll, Pitch & Yaw Input to Torque
  (Variables|Default|SetZAxis AxisValue)
  (Class|PrimitiveComponent|AddTorqueinDegrees (Variables|Default|GetCollision) (Math|Vector|Lerp(Vector) "0, 0, 0" (* (* AxisValue (Variables|Default|GetAirHandling)) (Math|Vector|GetUpVector (Variables|Default|GetCollision))) 0.1) "None" true))

(event Input|MouseEvents|LeftMouseButton
  (params (Key :type Key%20Structure :default "None"))
  (bind _skeletalmesh (Variables|Default|GetSkeletalMesh))
  (:Pressed
    (Game|SpawnActorfromClass "/Game/Blueprints/Bullet.Bullet_C" (Math|Conversions|ToTransform(Vector) (+ (Transformation|GetWorldLocation _skeletalmesh) (Math|Vector|GetForwardVector _skeletalmesh))) "Undefined" self 0)))

(fn ConstructionScript)

(fn ThrottleControl
  (bind _maxthrottle (Variables|Default|GetMaxThrottle))
  (bind _minthrottle (Variables|Default|GetMinThrottle))
  (if (Variables|Default|GetThrottleUP)
    (bind _result (Math|Integer|IncrementInt (Variables|Default|GetThrottle))
      (:%20%20
        (Variables|Default|SetThrottle (Math|Integer|Clamp(Integer) _result _minthrottle _maxthrottle))))
    (elif (Variables|Default|GetThrottleDOWN)
      (bind _result_2 (Math|Integer|DecrementInt (Variables|Default|GetThrottle))
        (:%20%20
          (Variables|Default|SetThrottle (Math|Integer|Clamp(Integer) _result_2 _minthrottle _maxthrottle)))))))

(fn CalculateSpeed
  (bind _collision (Variables|Default|GetCollision))
  (bind _returnvalue (Physics|GetPhysicsLinearVelocity _collision "None"))
  (Physics|SetPhysicsLinearVelocity _collision (Math|Vector|Lerp(Vector) _returnvalue (* (Math|Vector|GetForwardVector _collision) (Math|Integer|Clamp(Integer) (* (Variables|Default|GetThrottle) 25) 0 2500)) 0.01) false "None")
  (Variables|Default|SetSpeed (Math|Vector|Distance(Vector) "0, 0, 0" (Math|Vector|Lerp(Vector) _returnvalue (* (Math|Vector|GetForwardVector _collision) (Math|Integer|Clamp(Integer) (* (Variables|Default|GetThrottle) 25) 0 2500)) 0.01))))