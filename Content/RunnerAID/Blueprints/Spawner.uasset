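; Spawner is a vein track section for the ship runner that chains level generation and hosts enemies.
; A ship entering Box becomes linked to the section and, after a delay, requests the next one; passed sections expire once the ship is far away.
; Mesh hits damage the ship with a short cooldown.
; SpawnEnemy creates an enemy at End and slides it backward along CenterSpline using a slow, reversed timeline.
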(event OnComponentBeginOverlap(Box)
  (params (OverlappedComponent :type Primitive%20Component%20Object%20Reference) (OtherActor :type Actor%20Object%20Reference) (OtherComp :type Primitive%20Component%20Object%20Reference) (OtherBodyIndex :type Integer) (bFromSweep :type Boolean) (SweepResult :type Hit%20Result%20Structure%20%28by%20ref%29))
  (Development|PrintString (Utilities|String|Append (Utilities|GetObjectName OtherActor) ": overlap :" (Utilities|GetObjectName self)) true true "(R=0.000000,G=0.660000,B=1.000000,A=1.000000)" 5.0)
  (bind _asship (Utilities|Casting|CastToShip OtherActor)
    (:then
      (if (not (Variables|Default|GetPassed))
        (bind _output_get (Variables|Default|SetShipRef _asship))
        (Variables|/Game/RunnerAID/Blueprints/Ship.Ship_C|SetCurrentVeinSection _output_get self)
        (Utilities|FlowControl|Delay 1.0)
        (Default|CallSpawnNextSection _output_get)
        (Variables|Default|SetPassed true)
        (Utilities|FlowControl|Delay 1.0)))
    (:CastFailed
      (Development|PrintString "Failed to set ship ref in vein spawned"))))

(event OnComponentBeginOverlap(MidOverlap)
  (params (OverlappedComponent :type Primitive%20Component%20Object%20Reference) (OtherActor :type Actor%20Object%20Reference) (OtherComp :type Primitive%20Component%20Object%20Reference) (OtherBodyIndex :type Integer) (bFromSweep :type Boolean) (SweepResult :type Hit%20Result%20Structure%20%28by%20ref%29))
  (if (== (Utilities|GetClass OtherActor) "/Game/RunnerAID/Blueprints/Ship.Ship_C")
    (Utilities|Casting|CastToShip OtherActor
      (:then
        (Variables|Default|SetisCurrentlyOverlapping true))
      (:CastFailed
        (Development|PrintString "Failed to set ship ref in vein spawned")))))

(event OnComponentEndOverlap(MidOverlap)
  (params (OverlappedComponent :type Primitive%20Component%20Object%20Reference) (OtherActor :type Actor%20Object%20Reference) (OtherComp :type Primitive%20Component%20Object%20Reference) (OtherBodyIndex :type Integer))
  (if (== (Utilities|GetClass OtherActor) "/Game/RunnerAID/Blueprints/Ship.Ship_C")
    (Utilities|Casting|CastToShip OtherActor
      (:then
        (Variables|Default|SetisCurrentlyOverlapping false))
      (:CastFailed
        (Development|PrintString "Failed to set ship ref in vein spawned")))))

(event OnComponentHit(StaticMesh)
  (params (HitComponent :type Primitive%20Component%20Object%20Reference) (OtherActor :type Actor%20Object%20Reference) (OtherComp :type Primitive%20Component%20Object%20Reference) (NormalImpulse :type Vector :default "0, 0, 0") (Hit :type Hit%20Result%20Structure%20%28by%20ref%29))
  (Development|PrintString (Utilities|String|Append (Utilities|GetDisplayName OtherActor) " hit"))
  (bind _asship (Utilities|Casting|CastToShip OtherActor))
  (Utilities|FlowControl|DoOnce false :!label _label
    (:Completed
      (Game|Damage|ApplyDamage _asship 1.0 (Game|GetInstigatorController _asship) self "/Script/Engine.DamageType")
      (Utilities|FlowControl|Delay 0.2)
      (goto _label Reset))))

(event Custom|Spawn%20Enemy
  (params (Difficulty :type Integer))
  (bind _centerspline (Variables|Default|GetCenterSpline))
  (bind _returnvalue (Game|SpawnActorfromClass "/Game/RunnerAID/Blueprints/Enemy.Enemy_C" (Math|Transform|MakeTransform (Transformation|GetWorldLocation (Variables|Default|Getend)) "0, 0, 0" "1.000000,1.000000,1.000000") "AdjustIfPossibleButAlwaysSpawn" self 5 0))
  (Variables|Default|SetEnemy%20Ref _returnvalue)
  (Components|Timeline|SetPlayRate (Variables|Default|GetEnemyDrift) 0.05)
  (bind _driftlength (Timeline|EnemyDrift ReverseFromEnd)
    (:Update
      (bind _enemy_ref (Variables|Default|GetEnemy%20Ref)
        (:then
          (Transformation|SetActorLocation _enemy_ref (Spline|GetLocationatDistanceAlongSpline _centerspline (Math|Float|Lerp 0.0 (Spline|GetDistanceAlongSplineatSplinePoint _centerspline (- (Spline|GetNumberOfSplinePoints _centerspline) 1)) _driftlength) "World") false false))
        (:else
          (Timeline|EnemyDrift Stop))))))

(event EventTick
  (params (DeltaSeconds :type Float%20%28single-precision%29))
  (Utilities|FlowControl|Sequence
    (:then_0
      (if (Variables|Default|GetisCurrentlyOverlapping)
        (Development|PrintString (Utilities|String|Append "Current Section : " (Utilities|GetObjectName self)) true true "(R=1.000000,G=1.000000,B=1.000000,A=1.000000)" DeltaSeconds)))
    (:then_1
      (if (Variables|Default|GetPassed)
        (if (> (Transformation|GetDistanceTo self (Variables|Default|GetShipRef)) 2e+04)
          (Utilities|FlowControl|DoOnce false
            (:Completed
              (Actor|SetLifeSpan 15.0))))))))

(fn ConstructionScript)