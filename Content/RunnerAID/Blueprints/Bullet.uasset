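; Bullet projectile that a spawning owner fires, exploding on impact and damaging enemies.
; On spawn it launches its mesh with a velocity impulse along the owner's forward vector, scaled by owner speed, and sets a limited lifespan.
; Mesh hits branch on exact class: Ship and Spawner only trigger the explosion and destruction, while Enemy also takes damage.
; DoOnce gates guard each response against repeated hits.
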(event OnComponentHit(BulletMesh)
  (params (HitComponent :type Primitive%20Component%20Object%20Reference) (OtherActor :type Actor%20Object%20Reference) (OtherComp :type Primitive%20Component%20Object%20Reference) (NormalImpulse :type Vector :default "0, 0, 0") (Hit :type Hit%20Result%20Structure%20%28by%20ref%29))
  (bind _returnvalue (Utilities|GetClass OtherActor))
  (bind _self self)
  ;[1 1 1] CAST TO ENEMY CLASS CODE AHEAD
  (if (== _returnvalue "/Game/RunnerAID/Blueprints/Ship.Ship_C")
    (Utilities|FlowControl|DoOnce false
      (:Completed
        (Effects|SpawnEmitteratLocation "/Game/StarterContent/Particles/P_Explosion.P_Explosion" "0, 0, 0" "0, 0, 0" "0.700000,0.700000,0.700000" true "AutoRelease")
        (Actor|DestroyActor)))
    (elif (== _returnvalue "/Game/RunnerAID/Blueprints/Spawner.Spawner_C")
      (Utilities|Casting|CastToSpawner OtherActor
        (:then
          (Utilities|FlowControl|DoOnce false :!label _label
            (:Completed
              (Effects|SpawnEmitteratLocation "/Game/StarterContent/Particles/P_Explosion.P_Explosion" (.impactpoint Hit) "0, 0, 0" "0.700000,0.700000,0.700000" true "AutoRelease")
              (Actor|DestroyActor))))
        (:CastFailed
          (goto _label Reset)))
      (elif (== _returnvalue "/Game/RunnerAID/Blueprints/Enemy.Enemy_C")
        (Development|PrintString "BULLET HIT ENEMY")
        (Class|PrimitiveComponent|SetAllPhysicsLinearVelocity (Variables|Default|GetBulletMesh) "0, 0, 0" false)
        (bind _asenemy (Utilities|Casting|CastToEnemy OtherActor)
          (:then
            (Utilities|FlowControl|DoOnce false :!label _label_2
              (:Completed
                (Game|Damage|ApplyDamage _asenemy 5.0 (Game|GetInstigatorController _self) _self)
                (Effects|SpawnEmitteratLocation "/Game/StarterContent/Particles/P_Explosion.P_Explosion" (.impactpoint Hit) "0, 0, 0" "0.700000,0.700000,0.700000" true "AutoRelease")
                (Actor|DestroyActor))))
          (:CastFailed
            (goto _label_2 Reset)))))))

(event EventBeginPlay
  (bind _returnvalue (Components|GetOwner))
  ;[1 1 1] Bullet Movement
  (Actor|SetLifeSpan 1e+01)
  (Physics|AddImpulse (Variables|Default|GetBulletMesh) (* (Transformation|GetActorForwardVector _returnvalue) (Math|Vector|VectorLength (Transformation|GetVelocity _returnvalue)) 2e+01) "None" true)
  (Development|PrintString "Pew"))

(event Collision|EventActorBeginOverlap
  (params (OtherActor :type Actor%20Object%20Reference)))

(event EventTick
  (params (DeltaSeconds :type Float%20%28single-precision%29)))

(fn ConstructionScript)