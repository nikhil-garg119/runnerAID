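; Enemy actor that circles its pivot and expires after a fixed lifespan, acting as a shootable hazard for the Ship.
; A looping roll timeline swings the offset mesh around, with speed and offset randomized in the construction script.
; AnyDamage lowers Health and records the instigator, while Tick polls for death to explode and award score, noting Bullet kills.
; Ship overlap explodes it, damages the Ship and deducts score, more heavily for Bloodrunner component hits.
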(event OnComponentBeginOverlap(StaticMesh)
  (params (OverlappedComponent :type Primitive%20Component%20Object%20Reference) (OtherActor :type Actor%20Object%20Reference) (OtherComp :type Primitive%20Component%20Object%20Reference) (OtherBodyIndex :type Integer) (bFromSweep :type Boolean) (SweepResult :type Hit%20Result%20Structure%20%28by%20ref%29))
  (bind _staticmesh (Variables|Default|GetStaticMesh))
  (bind _returnvalue (Transformation|GetWorldTransform _staticmesh))
  ;[1 0.3668 0.1514] Ship Hit Enemy
  (if (== (Utilities|GetClass OtherActor) "/Game/RunnerAID/Blueprints/Ship.Ship_C")
    (bind _asship (Utilities|Casting|CastToShip OtherActor)
      (:then
        (Utilities|FlowControl|DoOnce false :!label _label
          (:Completed
            (Effects|SpawnEmitteratLocation "/Game/StarterContent/Particles/P_Explosion.P_Explosion" (.location _returnvalue) (.rotation _returnvalue) (.scale _returnvalue) true "AutoRelease")
            (Game|Damage|ApplyDamage _asship 1e+01 (Game|GetInstigatorController _asship) self)
            (Actor|DestroyActor)
            (if (== (Variables|/Game/RunnerAID/Blueprints/Ship.Ship_C|Getbloodrunner _asship) OtherComp)
              (Audio|PlaySound2D "/Game/Interface_And_Item_Sounds/WAV/Error_Buzz_03.Error_Buzz_03" 1.0 1.0 0.0 0 0)
              (Default|PenaltyScore _asship 5)
              (else
                (Audio|PlaySoundatLocation "/Game/Interface_And_Item_Sounds/WAV/mixkit-arrow-whoosh-1491.mixkit-arrow-whoosh-1491" (.location _returnvalue) "0, 0, 0" 0.5 1.0 0.0 0 0 0 0)
                (Default|PenaltyScore _asship 1))))))
      (:CastFailed
        (goto _label Reset)))))

(event Custom|StartRevolve
  ;[0.1205 1 0.4249] Ambient Revolving
  (bind _lineartime (Timeline|RevolveTimeline Play)
    (:Update
      (Transformation|SetActorRelativeRotation (Math|Rotator|MakeRotator (* _lineartime 3.6e+02) 0.0 0.0)))))

(event Custom|Stop%20Revolve
  ;[0.1205 1 0.4249] Ambient Revolving
  (bind _lineartime (Timeline|RevolveTimeline Stop)
    (:Update
      (Transformation|SetActorRelativeRotation (Math|Rotator|MakeRotator (* _lineartime 3.6e+02) 0.0 0.0)))))

(event Custom|PrintDebug
  (params (Delta%20seconds :type Float%20%28double-precision%29))
  (Development|PrintString (Utilities|String|ToString(Vector) (Transformation|GetActorLocation)) true true "(R=0.000000,G=0.660000,B=1.000000,A=1.000000)" Delta%20seconds))

(event EventBeginPlay
  ;[1 0.1182 0.5808] Spawn & Death
  (CallFunction|StartRevolve)
  (Actor|SetLifeSpan 3e+01))

(event Game|Damage|EventAnyDamage
  (params (Damage :type Float%20%28single-precision%29) (DamageType :type Damage%20Type%20Object%20Reference) (InstigatedBy :type Controller%20Object%20Reference) (DamageCauser :type Actor%20Object%20Reference))
  ;[1 0.1689 0.139] Enemy Damaged
  (if (>= (Variables|Default|GetHealth) 0)
    (Variables|Default|SetHealth (Math|Float|Truncate (- (Variables|Default|GetHealth) Damage)))
    (Variables|Default|SetShot? (== (Utilities|GetClass DamageCauser) "/Game/RunnerAID/Blueprints/Bullet.Bullet_C"))
    (Variables|Default|SetDamageInstigator (Pawn|GetControlledPawn InstigatedBy))))

(event EventTick
  (params (DeltaSeconds :type Float%20%28single-precision%29))
  (bind _staticmesh (Variables|Default|GetStaticMesh))
  (bind _returnvalue (Transformation|GetWorldTransform _staticmesh))
  ;[1 0.1182 0.5808] Spawn & Death
  (CallFunction|PrintDebug DeltaSeconds)
  (if (>= 0 (Variables|Default|GetHealth))
    (Utilities|FlowControl|DoOnce false :!label _label
      (:Completed
        (Effects|SpawnEmitteratLocation "/Game/StarterContent/Particles/P_Explosion.P_Explosion" (.location _returnvalue) (.rotation _returnvalue) (.scale _returnvalue))
        (Actor|DestroyActor)
        (bind _asship (Utilities|Casting|CastToShip (Variables|Default|GetDamageInstigator))
          (:then
            (Default|AddtoScore _asship (Variables|Default|GetShot?)))
          (:CastFailed
            (Development|PrintString "Enemy destroy - cast to ship invalid")))))
    (else
      (goto _label Reset))))

(fn ConstructionScript
  (bind _returnvalue (Math|Random|RandomFloat))
  (bind _returnvalue_2 (* _returnvalue 3e+02))
  (bind _returnvalue_3 (+ _returnvalue_2 1.5e+02))
  (Components|Timeline|SetPlayRate (Variables|Default|GetRevolveTimeline) (* (+ _returnvalue 0.5) 0.1))
  (Transformation|SetRelativeLocation (Variables|Default|GetStaticMesh) (Math|Vector|MakeVector 0.0 _returnvalue_3 _returnvalue_3) false false))