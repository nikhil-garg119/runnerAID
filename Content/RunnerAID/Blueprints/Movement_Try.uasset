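; Experimental runner pawn that pushes itself forward every tick, fires bullets on left click and loses health on any overlap.
; Roll and pitch inputs apply clamped, lerped rotations using SmoothLerp alphas, though the pitch target is left unwired.
; SpawnVein loops on a delay, replacing the previous Spawner with one at its End transform.
; Mouse_Movement is never called here, and death only prints when health equals exactly zero.
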(event Custom|MoveForward
  (params (DeltaSeconds :type Float%20%28double-precision%29))
  ;[1 1 1] Forward Movement
  (Pawn|Input|AddMovementInput (Math|Vector|GetForwardVector (Transformation|GetWorldRotation (Variables|Collision|GetCapsuleComponent))) (Variables|Default|GetForward_Velocity) true))

(event Custom|Mouse_Movement
  ;[1 1 1] Mouse Movement
  (bind _returnvalue (Class|WidgetLayoutLibrary|GetMousePositiononViewport))
  (bind _sweephitresult (Transformation|SetActorLocation (Math|Vector|MakeVector (.X (Math|Vector|BreakVector (Transformation|GetWorldLocation (Variables|Default|GetSkeletalMesh)))) (.X (Math|Vector2D|BreakVector2D _returnvalue)) (.Y (Math|Vector2D|BreakVector2D _returnvalue))) true false)))

(event Custom|SpawnVein
  (params (Spawn%20Transform :type Transform))
  (bind _veinspawn (Variables|Default|GetVeinSpawn)
    (:then
      (Actor|DestroyActor _veinspawn))
    (:else
      _))
  (bind _returnvalue (Game|SpawnActorfromClass "/Game/RunnerAID/Blueprints/Spawner.Spawner_C" Spawn%20Transform "Undefined" 0 0))
  (bind _output_get (Variables|Default|SetVeinSpawn _returnvalue))
  (Class|Actor|AddActorWorldRotation _output_get "0, 0, 0")
  (Development|PrintString (Utilities|String|ToString(Vector) (Transformation|GetWorldLocation (Variables|/Game/RunnerAID/Blueprints/Spawner.Spawner_C|Getend _returnvalue))) true true "(R=0.000000,G=0.000000,B=0.000000,A=1.000000)")
  (bind _output_get_2 (Variables|Default|SetNewTransform (Math|Transform|MakeTransform (Transformation|GetWorldLocation (Variables|/Game/RunnerAID/Blueprints/Spawner.Spawner_C|Getend _returnvalue)) (Transformation|GetWorldRotation (Variables|/Game/RunnerAID/Blueprints/Spawner.Spawner_C|Getend _returnvalue)))))
  (Utilities|FlowControl|Delay 5.0)
  (CallFunction|SpawnVein _output_get_2))

(event Custom|OnDeath
  ;[1 1 1] OnDeath
  (if (== (Variables|Default|GetHealth) 0.0)
    (Development|PrintString "Dead")))

(event EventBeginPlay
  (Input|EnableInput (Game|GetPlayerController 0))
  (Development|PrintString "Input enabled")
  (CallFunction|SpawnVein (Math|Transform|MakeTransform "0, 0, 0")))

(event EventTick
  (params (DeltaSeconds :type Float%20%28single-precision%29))
  (bind _lerp_variable_out (Utilities|SmoothLerp (Variables|Default|GetLerpRollVar) (Variables|Default|GetRoll%20Rate)))
  (Variables|Default|SetLerpRollVar _lerp_variable_out)
  (bind _lerp_variable_out_2 (Utilities|SmoothLerp (Variables|Default|GetLerpPitchVar) (Variables|Default|GetPitch%20Rate)))
  (Variables|Default|SetLerpPitchVar _lerp_variable_out_2)
  (CallFunction|MoveForward DeltaSeconds)
  (CallFunction|OnDeath))

(event Collision|EventActorBeginOverlap
  (params (OtherActor :type Actor%20Object%20Reference))
  ;[1 1 1] Taking Damage From Collisions
  (Variables|Default|SetHealth (- (Variables|Default|GetHealth) 15.0)))

(event Input|AxisEvents|InputAxisPitch
  (params (AxisValue :type Float%20%28single-precision%29))
  (bind _skeletalmesh (Variables|Default|GetSkeletalMesh))
  (bind _relativerotation (Variables|/Script/Engine.SceneComponent|GetRelativeRotation _skeletalmesh))
  ;[1 1 1] Rotation
  (Development|PrintString (Utilities|String|ToString(Rotator) _relativerotation))
  (if (<= (Math|Float|Absolute(Float) (+ (* AxisValue (Variables|Default|GetPitch%20Rate)) (.Pitch (Math|Rotator|BreakRotator _relativerotation)))) 3e+01)
    (Transformation|SetActorRelativeRotation self (Math|Rotator|Lerp(Rotator) (Transformation|GetWorldRotation (Variables|Collision|GetCapsuleComponent)) "0, 0, 0" (Variables|Default|GetLerpPitchVar)))))

(event Input|AxisEvents|InputAxisRoll
  (params (AxisValue :type Float%20%28single-precision%29))
  (bind _roll_rate (Variables|Default|GetRoll%20Rate))
  (bind _skeletalmesh (Variables|Default|GetSkeletalMesh))
  (bind _returnvalue (Transformation|GetWorldRotation _skeletalmesh))
  (bind _returnvalue_2 (* AxisValue _roll_rate))
  (bind _roll (Math|Rotator|BreakRotator _returnvalue))
  (bind _returnvalue_3 (+ _returnvalue_2 _roll))
  ;[1 1 1] Rotation
  (if (<= (Math|Float|Absolute(Float) _returnvalue_3) 9e+01)
    (Transformation|SetRelativeRotation (Variables|Default|GetSkeletalMesh) (Math|Rotator|Lerp(Rotator) _returnvalue (Math|Rotator|MakeRotator _returnvalue_3 0.0 0.0) (Variables|Default|GetLerpRollVar)) false false)))

(event Input|MouseEvents|LeftMouseButton
  (params (Key :type Key%20Structure))
  ;[1 1 1] Shooting
  (:Pressed
    (Audio|SpawnSound2D 0 1.0 1.0 0.0 0)
    (Game|SpawnActorfromClass "/Game/RunnerAID/Blueprints/Bullet.Bullet_C" (Transformation|GetWorldTransform (Variables|Default|GetSkeletalMesh)) "Undefined" 0 0)
    (Development|PrintString "Hello")))

(fn ConstructionScript)