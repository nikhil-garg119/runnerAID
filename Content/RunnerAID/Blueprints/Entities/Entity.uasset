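; Entity actor that revolves ambiently and can drift along the spline of its parent vein, expiring after 30 seconds.
; Construction randomizes the mesh's Y/Z offset and revolve speed, so a timeline rolling the actor swings the mesh around its origin.
; StartDrift plays a rate-adjustable timeline in reverse, moving the actor from the spline's end toward its start.
; Debug strings print its location every tick and announce drift starts.
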(event Custom|StartRevolve
  ;[0.1205 1 0.4249] Ambient Revolving
  (bind _lineartime (Timeline|RevolveTimeline Play)
    (:Update
      (Transformation|SetActorRelativeRotation (Math|Rotator|MakeRotator (* _lineartime 3.6e+02) 0.0 0.0)))))

(event Custom|Stop%20Revolve
  ;[0.1205 1 0.4249] Ambient Revolving
  (bind _lineartime (Timeline|RevolveTimeline Stop)
    (:Update
      (Transformation|SetActorRelativeRotation (Math|Rotator|MakeRotator (* _lineartime 3.6e+02) 0.0 0.0)))))

(event Custom|PrintDebug
  (params (Delta%20seconds :type Float%20%28double-precision%29))
  ;[1 1 1] Print debug
  (Development|PrintString (Utilities|String|ToString(Vector) (Transformation|GetActorLocation)) true true "(R=0.000000,G=0.660000,B=1.000000,A=1.000000)" Delta%20seconds))

(event Custom|Start%20Drift
  (params (Play%20Rate :type Float%20%28double-precision%29))
  (bind _parentvein (Variables|Default|GetParentVein))
  (bind _centerspline (Variables|/Game/RunnerAID/Blueprints/VeinSection.VeinSection_C|GetCenterSpline _parentvein))
  ;[0.4311 1 0.1624] Drift Along Vein
  (Development|PrintString (Utilities|String|Append (Utilities|GetObjectName self) " : Drift Start") true true "(R=0.092771,G=0.181128,B=1.000000,A=1.000000)" 5.0)
  (Components|Timeline|SetPlayRate (Variables|Default|GetDrift%20Along%20Vein) Play%20Rate)
  (bind _drift (Timeline|Drift%20Along%20Vein ReverseFromEnd)
    (:Update
      (Transformation|SetActorLocation (Spline|GetLocationatDistanceAlongSpline _centerspline (Math|Float|Lerp 0.0 (Spline|GetDistanceAlongSplineatSplinePoint _centerspline (- (Spline|GetNumberOfSplinePoints _centerspline) 1)) _drift) "World") false false))))

(event EventBeginPlay
  ;[1 0.1182 0.5808] Spawn & Death
  (CallFunction|StartRevolve)
  (Actor|SetLifeSpan 3e+01))

(event EventTick
  (params (DeltaSeconds :type Float%20%28single-precision%29))
  ;[1 0.1182 0.5808] Spawn & Death
  (CallFunction|PrintDebug DeltaSeconds))

(fn ConstructionScript
  (bind _returnvalue (Math|Random|RandomFloat))
  (bind _returnvalue_2 (* _returnvalue 3e+02))
  (bind _returnvalue_3 (+ _returnvalue_2 1.5e+02))
  (Components|Timeline|SetPlayRate (Variables|Default|GetRevolveTimeline) (* (+ _returnvalue 0.5) 0.1))
  (Transformation|SetRelativeLocation (Variables|Default|GetStaticMesh) (Math|Vector|MakeVector 0.0 _returnvalue_3 _returnvalue_3) false false))