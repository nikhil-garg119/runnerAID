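; Player ship pawn for an endless vein-tunnel runner, also owning menus, HUD, pause, scoring and game over.
; Physics flight applies input torque and blends velocity toward forward times throttle, which drives thrust VFX and audio.
; It chains randomly rotated VeinSections end to start, raising minimum throttle with distance.
; It handles auto-fire, crosshair projection and shield-before-health damage, plus a timeline spline autopilot for the menu and debugging.
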(event OnComponentBeginOverlap(DestroyBarrier)
  (params (OverlappedComponent :type Primitive%20Component%20Object%20Reference) (OtherActor :type Actor%20Object%20Reference) (OtherComp :type Primitive%20Component%20Object%20Reference) (OtherBodyIndex :type Integer) (bFromSweep :type Boolean) (SweepResult :type Hit%20Result%20Structure%20%28by%20ref%29))
  ;[1 0.1182 0.5808] Destroy Barrier
  (bind _asenemy (Utilities|Casting|CastToEnemy OtherActor)
    (:then
      (Utilities|IsValid _asenemy
        (:Is%20Valid
          (Utilities|FlowControl|DoOnce false :!label _label
            (:Completed
              (Development|PrintString "BARRIER DESTROYED ENEMY" true true "(R=0.000000,G=1.000000,B=0.021866,A=1.000000)")
              (if (not (Game|IsActorBeingDestroyed _asenemy))
                (Actor|DestroyActor _asenemy)
                (goto _label Reset)))))
        (:Is%20Not%20Valid
          (goto _label Reset))))
    (:CastFailed
      (goto _label Reset))))

(event Custom|SpawnVein
  (params (Spawn%20Transform :type Transform))
  (bind _veinsections (Variables|Default|GetVeinSections))
  ;[1 0.1182 0.5808] Spawning Tunnel Veins
  (Development|PrintString (Utilities|String|ToString(Transform) Spawn%20Transform))
  (bind _returnvalue (Game|SpawnActorfromClass "/Game/RunnerAID/Blueprints/VeinSection.VeinSection_C" Spawn%20Transform "AlwaysSpawn" 0 0))
  (Game|AssignOnDestroyed _returnvalue (delegate Custom|onDestroyedVeinSection))
  (Default|SpawnEnemy _returnvalue)
  (Utilities|Array|AddUnique _veinsections _returnvalue)
  (if (Variables|Default|GetRandomRotate)
    (Math|Integer|IncrementInt (Variables|Default|GetVeinCount)
      (:%20%20
        (Class|Actor|AddActorWorldRotation _returnvalue (Math|Vector|RotatorfromAxisandAngle (Math|Vector|GetForwardVector (Variables|/Game/RunnerAID/Blueprints/VeinSection.VeinSection_C|Getstart _returnvalue)) (Math|Random|RandomFloatinRange 0.0 1.8e+02)))))
    (else
      (bind _output_get (Variables|Default|SetCurrentVeinSection _returnvalue))
      (Actor|SetLifeSpan _output_get 2e+01)))
  (Development|PrintString (Utilities|String|Append (Utilities|GetObjectName _returnvalue) ": " (Utilities|String|ToString(Vector) (Transformation|GetWorldLocation (Variables|/Game/RunnerAID/Blueprints/VeinSection.VeinSection_C|Getend _returnvalue))) " : Length :: " (Utilities|String|ToString(Integer) (Utilities|Array|Length _veinsections))) true true "(R=0.170833,G=0.170833,B=0.170833,A=1.000000)" 4.0)
  (Variables|Default|SetNext%20Transform (Math|Transform|MakeTransform (Transformation|GetWorldLocation (Variables|/Game/RunnerAID/Blueprints/VeinSection.VeinSection_C|Getend _returnvalue)) (Transformation|GetWorldRotation (Variables|/Game/RunnerAID/Blueprints/VeinSection.VeinSection_C|Getend _returnvalue))))
  (Variables|Default|SetRandomRotate true)
  (CallFunction|LimitThrottle))

(event Custom|Spawn%20Next
  ;[0.1381 1 0.1663] Setup
  (CallFunction|SpawnVein (Variables|Default|GetNext%20Transform)))

(event Custom|StartMainMenu
  (bind _returnvalue (Game|GetPlayerController 0))
  ;[0.4943 0.09617 1] Debug Modes
  (Widget|SetVisibility (Variables|Default|GetinGameWidget) "Hidden")
  (Widget|SetVisibility (Variables|Default|GetMainMenu) "Visible")
  (Collision|SetCollisionEnabled (Variables|Default|GetCollision) "QueryOnly")
  (CallFunction|Autopilot)
  (Rendering|SetVisibility (Variables|Default|GetCollision) false false)
  (Input|SetInputModeUIOnly _returnvalue (Variables|Default|GetMainMenu) "DoNotLock")
  (Variables|/Script/Engine.PlayerController|SetbShowMouseCursor _returnvalue true))

(event Custom|SpawnThrustSFX
  (bind _thrustvfx (Variables|Default|GetThrustVFX))
  (bind _throttle (Variables|Default|GetThrottle))
  (bind _maxthrottle (Variables|Default|GetMaxThrottle))
  (bind _returnvalue (/ _throttle _maxthrottle))
  (bind _returnvalue_2 (+ _returnvalue 0.45))
  ;[0.1063 1 0.7015] Thrust SFX
  (bind _as_game_main_mode (Variables|Default|GetAs%20Game%20Main%20Mode)
    (:then
      (Audio|SpawnSoundAttached "/Game/Interface_And_Item_Sounds/WAV/thrustsound.thrustsound" _thrustvfx "None" "0, 0, 0" "0, 0, 0" "KeepRelativeOffset" true (* (Variables|/Game/RunnerAID/Blueprints/GameMainMode.GameMainMode_C|GetSFXVolume _as_game_main_mode) _returnvalue_2) _returnvalue_2 0.0 0 0)
      (Utilities|FlowControl|Delay 0.99)
      (Audio|SpawnSoundAttached "/Game/Interface_And_Item_Sounds/WAV/thrustsound.thrustsound" _thrustvfx "None" "0, 0, 0" "0, 0, 0" "KeepRelativeOffset" true (* (Variables|/Game/RunnerAID/Blueprints/GameMainMode.GameMainMode_C|GetSFXVolume _as_game_main_mode) _returnvalue_2) _returnvalue_2 0.0 0 0))
    (:else)))

(event Custom|StartMoveAlongSpline
  (bind _veinsections (Variables|Default|GetVeinSections))
  ;[1 0.1689 0.139] Move Along Spline
  (bind _pos (Timeline|SplineTimeline PlayFromStart)
    (:Update
      (bind _currentveinsection (Variables|Default|GetCurrentVeinSection)
        (:then
          (Utilities|FlowControl|Sequence
            (:then_0
              (if (> (+ _pos (Variables|Default|GetDistAlongVein)) 0.99)
                (bind _result (Math|Integer|IncrementInt (Utilities|Array|FindItem _veinsections _currentveinsection))
                  (:%20%20
                    (bind (_array_element _array_index) (Utilities|Array|ForEachLoopwithBreak _veinsections)
                      (:LoopBody
                        (if (== _array_index _result)
                          (Utilities|IsValid _array_element
                            (:Is%20Valid
                              (bind _output_get (Variables|Default|SetNextVeinSection _array_element))
                              (bind _output_get_2 (Variables|Default|SetNextSectionName (Utilities|String|Append "NEXT SECTION NAME : " (Utilities|GetObjectName _output_get))))
                              (Development|PrintString _output_get_2 true true "(R=0.000000,G=1.000000,B=0.032689,A=1.000000)" 5.0)
                              (bind _nextveinsection (Variables|Default|GetNextVeinSection)
                                (:then
                                  (Variables|Default|SetCurrentVeinSection _nextveinsection)
                                  (Variables|Default|SetDistAlongVein 0.0)
                                  (CallFunction|StartMoveAlongSpline))
                                (:else)))
                            (:Is%20Not%20Valid
                              (Development|PrintString "Next section not valid ===" true true "(R=1.000000,G=0.006772,B=0.000000,A=1.000000)" 1e+01))))))))
                (else
                  (Components|MoveComponentTo (Variables|Transformation|GetRootComponent) (Spline|GetLocationatDistanceAlongSpline (Variables|/Game/RunnerAID/Blueprints/VeinSection.VeinSection_C|GetCenterSpline _currentveinsection) (+ (Math|Float|Lerp 0.0 (Spline|GetDistanceAlongSplineatSplinePoint (Variables|/Game/RunnerAID/Blueprints/VeinSection.VeinSection_C|GetCenterSpline _currentveinsection) (- (Spline|GetNumberOfSplinePoints (Variables|/Game/RunnerAID/Blueprints/VeinSection.VeinSection_C|GetCenterSpline _currentveinsection)) 1)) (+ _pos (Variables|Default|GetDistAlongVein))) 0.01) "World") (Math|Rotator|MakeRotator (* (Class|SplineComponent|GetRollatDistanceAlongSpline (Variables|/Game/RunnerAID/Blueprints/VeinSection.VeinSection_C|GetCenterSpline _currentveinsection) (+ (Math|Float|Lerp 0.0 (Spline|GetDistanceAlongSplineatSplinePoint (Variables|/Game/RunnerAID/Blueprints/VeinSection.VeinSection_C|GetCenterSpline _currentveinsection) (- (Spline|GetNumberOfSplinePoints (Variables|/Game/RunnerAID/Blueprints/VeinSection.VeinSection_C|GetCenterSpline _currentveinsection)) 1)) (+ _pos (Variables|Default|GetDistAlongVein))) 0.01) "World") (Math|Float|Clamp(Float) (- (+ _pos (Variables|Default|GetDistAlongVein)) (Math|Float|Square (+ _pos (Variables|Default|GetDistAlongVein)))))) (.pitch (Math|Conversions|RotationFromXVector (Spline|GetTangentatDistanceAlongSpline (Variables|/Game/RunnerAID/Blueprints/VeinSection.VeinSection_C|GetCenterSpline _currentveinsection) (+ (Math|Float|Lerp 0.0 (Spline|GetDistanceAlongSplineatSplinePoint (Variables|/Game/RunnerAID/Blueprints/VeinSection.VeinSection_C|GetCenterSpline _currentveinsection) (- (Spline|GetNumberOfSplinePoints (Variables|/Game/RunnerAID/Blueprints/VeinSection.VeinSection_C|GetCenterSpline _currentveinsection)) 1)) (+ _pos (Variables|Default|GetDistAlongVein))) 0.01) "World"))) (.yaw (Math|Conversions|RotationFromXVector (Spline|GetTangentatDistanceAlongSpline (Variables|/Game/RunnerAID/Blueprints/VeinSection.VeinSection_C|GetCenterSpline _currentveinsection) (+ (Math|Float|Lerp 0.0 (Spline|GetDistanceAlongSplineatSplinePoint (Variables|/Game/RunnerAID/Blueprints/VeinSection.VeinSection_C|GetCenterSpline _currentveinsection) (- (Spline|GetNumberOfSplinePoints (Variables|/Game/RunnerAID/Blueprints/VeinSection.VeinSection_C|GetCenterSpline _currentveinsection)) 1)) (+ _pos (Variables|Default|GetDistAlongVein))) 0.01) "World")))) true true 0.1 false))))))
        (:else
          (Development|PrintString "CURRENT VEIN SECTION CAST INVALID : Stopping move along spline")
          (CallFunction|StopMoveAlongSpline))))))

(event Custom|Start%20Game
  ;[0.4943 0.09617 1] Debug Modes
  (Variables|Default|SetVeinCount 0)
  (Variables|Default|SetHealth 100)
  (Variables|Default|SetShield 4)
  (Variables|Default|SetScore 0)
  (Variables|Default|SetinPlay? true)
  (Input|EnableInput (Game|GetPlayerController 0))
  (Widget|SetVisibility (Variables|Default|GetinGameWidget) "Visible")
  (Widget|SetVisibility (Variables|Default|GetMainMenu) "Hidden")
  (Collision|SetCollisionEnabled (Variables|Default|Getbloodrunner) "QueryAndPhysics")
  (CallFunction|StopMoveAlongSpline)
  (Game|SetGamePaused false)
  (Rendering|SetVisibility (Variables|Default|GetCollision) true true))

(event Custom|SetGamePause
  (params (Pause? :type Boolean))
  (bind _returnvalue (Game|GetPlayerController 0))
  (bind _ingamewidget (Variables|Default|GetinGameWidget))
  (bind _crosshair (Variables|Default|GetCrosshair))
  ;[0.08907 0.3929 1] Pause
  (if Pause?
    (Development|PrintString "Paused")
    (Widget|SetVisibility _crosshair "Hidden")
    (Default|SetPaused _ingamewidget true)
    (Input|SetInputModeGameandUI _returnvalue _ingamewidget "DoNotLock" true)
    (Variables|/Script/Engine.PlayerController|SetbShowMouseCursor _returnvalue true)
    (Utilities|FlowControl|DelayUntilNextTick)
    (Game|SetGamePaused true)
    (else
      (Widget|SetVisibility _crosshair "Visible")
      (Game|SetGamePaused false)
      (Default|SetPaused _ingamewidget false)
      (Input|SetInputModeGameOnly _returnvalue)
      (Variables|/Script/Engine.PlayerController|SetbShowMouseCursor _returnvalue false)
      (Input|SetInputModeGameOnly _returnvalue)
      (Development|PrintString "Unpaused"))))

(event Custom|Laser%20Point
  (bind _returnvalue (Transformation|GetActorLocation))
  (bind _returnvalue_2 (Game|GetPlayerController 0))
  (bind _self self)
  (bind _returnvalue_3 (Transformation|GetActorForwardVector _self))
  (bind _returnvalue_4 (* _returnvalue_3 3000))
  (bind _returnvalue_5 (+ _returnvalue _returnvalue_4))
  (bind (_screenlocation _returnvalue_6) (Class|PlayerController|ProjectWorldLocationtoScreen _returnvalue_2 _returnvalue_5 true))
  ;[0.884 0.07804 1] Laser Pointer
  (bind _outhit (Collision|LineTraceByChannel _returnvalue _returnvalue_5 "TraceTypeQuery1" true (Utilities|Array|MakeArray _self 0) "None"))
  (bind _crosshair (Variables|Default|GetCrosshair)
    (:then
      (if _returnvalue_6
        (Class|UserWidget|SetPositioninViewport _crosshair _screenlocation true)))
    (:else)))

(event Custom|GameOver
  ;[1 0.3668 0.1514] Game Over
  (Variables|Default|SetinPlay? false)
  (Game|SetGamePaused true)
  (Variables|/Script/Engine.PlayerController|SetbShowMouseCursor (Game|GetPlayerController 0) true)
  (Widget|SetVisibility (Variables|Default|GetCrosshair) "Hidden")
  (Default|DisplayGameOver (Variables|Default|GetinGameWidget))
  (Audio|PlaySound2D "/Game/Interface_And_Item_Sounds/WAV/Cartoon_Falling_05.Cartoon_Falling_05" 1.0 1.0 0.0 0 0)
  (Actor|DestroyActor)
  (Game|SetGamePaused true)
  (bind _asgame_main_mode (Utilities|Casting|CastToGameMainMode (Game|GetGameMode)))
  (Variables|/Game/RunnerAID/Blueprints/GameMainMode.GameMainMode_C|SetLast%20Score _asgame_main_mode (Variables|Default|GetScore)))

(event Custom|Autopilot
  ;[1 0.892 0.1503] Autopilot Initiate
  (Variables|Default|SetThrottle (/ (+ (Variables|Default|GetMaxThrottle) (Variables|Default|GetMinThrottle)) 2))
  (Components|Timeline|SetPlayRate (Variables|Default|GetSplineTimeline) (Variables|Default|GetAutopilot%20Play%20Speed))
  (CallFunction|MoveAlongSpline))

(event Custom|MoveAlongSpline
  (bind _veinsections (Variables|Default|GetVeinSections))
  ;[1 0.1689 0.139] Move Along Spline
  (CallFunction|CalcDistAlongVein)
  (bind _pos (Timeline|SplineTimeline PlayFromStart)
    (:Update
      (bind _currentveinsection (Variables|Default|GetCurrentVeinSection)
        (:then
          (Utilities|FlowControl|Sequence
            (:then_0
              (if (> (+ _pos (Variables|Default|GetDistAlongVein)) 0.99)
                (bind _result (Math|Integer|IncrementInt (Utilities|Array|FindItem _veinsections _currentveinsection))
                  (:%20%20
                    (bind (_array_element _array_index) (Utilities|Array|ForEachLoopwithBreak _veinsections)
                      (:LoopBody
                        (if (== _array_index _result)
                          (Utilities|IsValid _array_element
                            (:Is%20Valid
                              (bind _output_get (Variables|Default|SetNextVeinSection _array_element))
                              (bind _output_get_2 (Variables|Default|SetNextSectionName (Utilities|String|Append "NEXT SECTION NAME : " (Utilities|GetObjectName _output_get))))
                              (Development|PrintString _output_get_2 true true "(R=0.000000,G=1.000000,B=0.032689,A=1.000000)" 5.0)
                              (bind _nextveinsection (Variables|Default|GetNextVeinSection)
                                (:then
                                  (Variables|Default|SetCurrentVeinSection _nextveinsection)
                                  (Variables|Default|SetDistAlongVein 0.0)
                                  (CallFunction|StartMoveAlongSpline))
                                (:else)))
                            (:Is%20Not%20Valid
                              (Development|PrintString "Next section not valid ===" true true "(R=1.000000,G=0.006772,B=0.000000,A=1.000000)" 1e+01))))))))
                (else
                  (Components|MoveComponentTo (Variables|Transformation|GetRootComponent) (Spline|GetLocationatDistanceAlongSpline (Variables|/Game/RunnerAID/Blueprints/VeinSection.VeinSection_C|GetCenterSpline _currentveinsection) (+ (Math|Float|Lerp 0.0 (Spline|GetDistanceAlongSplineatSplinePoint (Variables|/Game/RunnerAID/Blueprints/VeinSection.VeinSection_C|GetCenterSpline _currentveinsection) (- (Spline|GetNumberOfSplinePoints (Variables|/Game/RunnerAID/Blueprints/VeinSection.VeinSection_C|GetCenterSpline _currentveinsection)) 1)) (+ _pos (Variables|Default|GetDistAlongVein))) 0.01) "World") (Math|Rotator|MakeRotator (* (Class|SplineComponent|GetRollatDistanceAlongSpline (Variables|/Game/RunnerAID/Blueprints/VeinSection.VeinSection_C|GetCenterSpline _currentveinsection) (+ (Math|Float|Lerp 0.0 (Spline|GetDistanceAlongSplineatSplinePoint (Variables|/Game/RunnerAID/Blueprints/VeinSection.VeinSection_C|GetCenterSpline _currentveinsection) (- (Spline|GetNumberOfSplinePoints (Variables|/Game/RunnerAID/Blueprints/VeinSection.VeinSection_C|GetCenterSpline _currentveinsection)) 1)) (+ _pos (Variables|Default|GetDistAlongVein))) 0.01) "World") (Math|Float|Clamp(Float) (- (+ _pos (Variables|Default|GetDistAlongVein)) (Math|Float|Square (+ _pos (Variables|Default|GetDistAlongVein)))))) (.pitch (Math|Conversions|RotationFromXVector (Spline|GetTangentatDistanceAlongSpline (Variables|/Game/RunnerAID/Blueprints/VeinSection.VeinSection_C|GetCenterSpline _currentveinsection) (+ (Math|Float|Lerp 0.0 (Spline|GetDistanceAlongSplineatSplinePoint (Variables|/Game/RunnerAID/Blueprints/VeinSection.VeinSection_C|GetCenterSpline _currentveinsection) (- (Spline|GetNumberOfSplinePoints (Variables|/Game/RunnerAID/Blueprints/VeinSection.VeinSection_C|GetCenterSpline _currentveinsection)) 1)) (+ _pos (Variables|Default|GetDistAlongVein))) 0.01) "World"))) (.yaw (Math|Conversions|RotationFromXVector (Spline|GetTangentatDistanceAlongSpline (Variables|/Game/RunnerAID/Blueprints/VeinSection.VeinSection_C|GetCenterSpline _currentveinsection) (+ (Math|Float|Lerp 0.0 (Spline|GetDistanceAlongSplineatSplinePoint (Variables|/Game/RunnerAID/Blueprints/VeinSection.VeinSection_C|GetCenterSpline _currentveinsection) (- (Spline|GetNumberOfSplinePoints (Variables|/Game/RunnerAID/Blueprints/VeinSection.VeinSection_C|GetCenterSpline _currentveinsection)) 1)) (+ _pos (Variables|Default|GetDistAlongVein))) 0.01) "World")))) true true 0.1 false))))))
        (:else
          (Development|PrintString "CURRENT VEIN SECTION CAST INVALID : Stopping move along spline")
          (CallFunction|StopMoveAlongSpline))))))

(event Custom|Add%20To%20Score
  (params (Shot? :type Boolean))
  ;[0.08907 0.3929 1] Scoring
  (if Shot?
    (Variables|Default|SetScore (+ (Variables|Default|GetScore) 5))
    (else
      (Math|Integer|IncrementInt (Variables|Default|GetScore)))))

(event Custom|StopMoveAlongSpline
  (bind _veinsections (Variables|Default|GetVeinSections))
  (bind _rootcomponent (Variables|Transformation|GetRootComponent))
  (bind _returnvalue (Transformation|GetWorldTransform _rootcomponent))
  ;[1 0.1689 0.139] Move Along Spline
  (Utilities|FlowControl|Sequence
    (:then_0
      (Transformation|SetActorLocationAndRotation (.location _returnvalue) (.rotation _returnvalue)))
    (:then_1
      (bind _pos (Timeline|SplineTimeline Stop)
        (:Update
          (bind _currentveinsection (Variables|Default|GetCurrentVeinSection)
            (:then
              (Utilities|FlowControl|Sequence
                (:then_0
                  (if (> (+ _pos (Variables|Default|GetDistAlongVein)) 0.99)
                    (bind _result (Math|Integer|IncrementInt (Utilities|Array|FindItem _veinsections _currentveinsection))
                      (:%20%20
                        (bind (_array_element _array_index) (Utilities|Array|ForEachLoopwithBreak _veinsections)
                          (:LoopBody
                            (if (== _array_index _result)
                              (Utilities|IsValid _array_element
                                (:Is%20Valid
                                  (bind _output_get (Variables|Default|SetNextVeinSection _array_element))
                                  (bind _output_get_2 (Variables|Default|SetNextSectionName (Utilities|String|Append "NEXT SECTION NAME : " (Utilities|GetObjectName _output_get))))
                                  (Development|PrintString _output_get_2 true true "(R=0.000000,G=1.000000,B=0.032689,A=1.000000)" 5.0)
                                  (bind _nextveinsection (Variables|Default|GetNextVeinSection)
                                    (:then
                                      (Variables|Default|SetCurrentVeinSection _nextveinsection)
                                      (Variables|Default|SetDistAlongVein 0.0)
                                      (CallFunction|StartMoveAlongSpline))
                                    (:else)))
                                (:Is%20Not%20Valid
                                  (Development|PrintString "Next section not valid ===" true true "(R=1.000000,G=0.006772,B=0.000000,A=1.000000)" 1e+01))))))))
                    (else
                      (Components|MoveComponentTo (Variables|Transformation|GetRootComponent) (Spline|GetLocationatDistanceAlongSpline (Variables|/Game/RunnerAID/Blueprints/VeinSection.VeinSection_C|GetCenterSpline _currentveinsection) (+ (Math|Float|Lerp 0.0 (Spline|GetDistanceAlongSplineatSplinePoint (Variables|/Game/RunnerAID/Blueprints/VeinSection.VeinSection_C|GetCenterSpline _currentveinsection) (- (Spline|GetNumberOfSplinePoints (Variables|/Game/RunnerAID/Blueprints/VeinSection.VeinSection_C|GetCenterSpline _currentveinsection)) 1)) (+ _pos (Variables|Default|GetDistAlongVein))) 0.01) "World") (Math|Rotator|MakeRotator (* (Class|SplineComponent|GetRollatDistanceAlongSpline (Variables|/Game/RunnerAID/Blueprints/VeinSection.VeinSection_C|GetCenterSpline _currentveinsection) (+ (Math|Float|Lerp 0.0 (Spline|GetDistanceAlongSplineatSplinePoint (Variables|/Game/RunnerAID/Blueprints/VeinSection.VeinSection_C|GetCenterSpline _currentveinsection) (- (Spline|GetNumberOfSplinePoints (Variables|/Game/RunnerAID/Blueprints/VeinSection.VeinSection_C|GetCenterSpline _currentveinsection)) 1)) (+ _pos (Variables|Default|GetDistAlongVein))) 0.01) "World") (Math|Float|Clamp(Float) (- (+ _pos (Variables|Default|GetDistAlongVein)) (Math|Float|Square (+ _pos (Variables|Default|GetDistAlongVein)))))) (.pitch (Math|Conversions|RotationFromXVector (Spline|GetTangentatDistanceAlongSpline (Variables|/Game/RunnerAID/Blueprints/VeinSection.VeinSection_C|GetCenterSpline _currentveinsection) (+ (Math|Float|Lerp 0.0 (Spline|GetDistanceAlongSplineatSplinePoint (Variables|/Game/RunnerAID/Blueprints/VeinSection.VeinSection_C|GetCenterSpline _currentveinsection) (- (Spline|GetNumberOfSplinePoints (Variables|/Game/RunnerAID/Blueprints/VeinSection.VeinSection_C|GetCenterSpline _currentveinsection)) 1)) (+ _pos (Variables|Default|GetDistAlongVein))) 0.01) "World"))) (.yaw (Math|Conversions|RotationFromXVector (Spline|GetTangentatDistanceAlongSpline (Variables|/Game/RunnerAID/Blueprints/VeinSection.VeinSection_C|GetCenterSpline _currentveinsection) (+ (Math|Float|Lerp 0.0 (Spline|GetDistanceAlongSplineatSplinePoint (Variables|/Game/RunnerAID/Blueprints/VeinSection.VeinSection_C|GetCenterSpline _currentveinsection) (- (Spline|GetNumberOfSplinePoints (Variables|/Game/RunnerAID/Blueprints/VeinSection.VeinSection_C|GetCenterSpline _currentveinsection)) 1)) (+ _pos (Variables|Default|GetDistAlongVein))) 0.01) "World")))) true true 0.1 false))))))
            (:else
              (Development|PrintString "CURRENT VEIN SECTION CAST INVALID : Stopping move along spline")
              (CallFunction|StopMoveAlongSpline))))))))

(event Custom|Limit%20Throttle
  ;[1 0.3668 0.1514] Throttle Limit
  (if (< (Variables|Default|GetMinThrottle) 99)
    (Variables|Default|SetMinThrottle (+ 10 (/ (Variables|Default|GetVeinCount) 10)))
    (if (< (Variables|Default|GetThrottle) (Variables|Default|GetMinThrottle))
      (Variables|Default|SetThrottle (Variables|Default|GetMinThrottle)))))

(event Custom|onDestroyedVeinSection
  (params (DestroyedActor :type Actor%20Object%20Reference))
  (bind _veinsections (Variables|Default|GetVeinSections))
  ;[1 0.1182 0.5808] Spawning Tunnel Veins
  (bind _asvein_section (Utilities|Casting|CastToVeinSection DestroyedActor))
  (if (Utilities|Array|ContainsItem _veinsections _asvein_section)
    (Utilities|Array|RemoveItem _veinsections _asvein_section)))

(event Custom|Penalty%20Score
  (params (Penalty%20Amount :type Integer))
  ;[0.08907 0.3929 1] Scoring
  (Variables|Default|SetScore (Math|Integer|SelectInt (- (Variables|Default|GetScore) Penalty%20Amount) 0 (> (- (Variables|Default|GetScore) Penalty%20Amount) 0))))

(event EventBeginPlay
  ;[0.1381 1 0.1663] Setup
  (Utilities|FlowControl|Sequence
    (:then_0
      (bind _asgame_main_mode (Utilities|Casting|CastToGameMainMode (Game|GetGameMode)))
      (Variables|Default|SetAs%20Game%20Main%20Mode _asgame_main_mode)
      (bind _returnvalue (UserInterface|CreateWidget "/Game/RunnerAID/Blueprints/Widgets/WBP_MainMenu.WBP_MainMenu_C" (Game|GetPlayerController 0)))
      (bind _output_get (Variables|Default|SetMainMenu _returnvalue))
      (UserInterface|Viewport|AddtoViewport _output_get 0)
      (Widget|SetVisibility _output_get "Visible")
      (bind _returnvalue_2 (UserInterface|CreateWidget "/Game/RunnerAID/Blueprints/Widgets/WBP_InGame.WBP_InGame_C" (Game|GetPlayerController 0)))
      (bind _output_get_2 (Variables|Default|SetinGameWidget _returnvalue_2))
      (UserInterface|Viewport|AddtoViewport _output_get_2 0)
      (Widget|SetVisibility _output_get_2 "Collapsed")
      (bind _returnvalue_3 (UserInterface|CreateWidget "/Game/RunnerAID/Blueprints/Widgets/WBP_HUD.WBP_HUD_C" (Game|GetPlayerController 0)))
      (bind _output_get_3 (Variables|Default|SetHUD _returnvalue_3))
      (UserInterface|Viewport|AddtoViewport _output_get_3 0)
      (Widget|SetVisibility _output_get_3 "Collapsed"))
    (:then_1
      (CallFunction|StartMainMenu)
      (EventDispatchers|BindEventtoSpawnNextSection (delegate Custom|Spawn%20Next))
      (Variables|Default|SetNext%20Transform (Math|Transform|MakeTransform "0, 0, 0" (Math|Vector|RotatorfromAxisandAngle (Transformation|GetActorUpVector self) 15.0)))
      (CallFunction|SpawnNext)
      (Utilities|FlowControl|Delay 1.0)
      (CallFunction|SpawnNext))))

(event EventTick
  (params (DeltaSeconds :type Float%20%28single-precision%29))
  (bind _returnvalue (Game|GetPlayerController 0))
  (bind _collision (Variables|Default|GetCollision))
  ;[0.09277 0.1811 1] Tick
  (Variables|Default|SetDelta%20Seconds DeltaSeconds)
  (if (Variables|Default|GetinPlay?)
    (Utilities|FlowControl|Sequence
      (:then_0
        (Utilities|FlowControl|DoOnce false :!label _label
          (:Completed
            (CallFunction|SpawnThrustSFX)
            (Utilities|Time|SetTimerbyFunctionName 0 "ThrottleControl" 0.05 true)
            (Utilities|Time|SetTimerbyFunctionName 0 "UpdateThrustVFX" 0.05 true 0.01)
            (Widget|SetVisibility (Variables|Default|GetHUD) "Visible")
            (Variables|/Script/Engine.PlayerController|SetbShowMouseCursor _returnvalue false)
            (bind _returnvalue_2 (UserInterface|CreateWidget "/Game/RunnerAID/Blueprints/Widgets/WBP_AIM.WBP_AIM_C" _returnvalue))
            (bind _output_get (Variables|Default|SetCrosshair _returnvalue_2))
            (UserInterface|Viewport|AddtoViewport _output_get 0)
            (Utilities|FlowControl|Delay 0.2)
            (Variables|Default|SetcanShoot true))))
      (:then_1
        (if (Class|PrimitiveComponent|IsPhysicsCollisionEnabled _collision)
          (Class|PrimitiveComponent|AddTorqueinDegrees _collision (/ (Math|Vector|NegateVector (Physics|GetPhysicsAngularVelocityinDegrees (Variables|Default|GetCollision) "None")) 0.5) "None" true)
          (Physics|AddForce _collision (Math|Vector|MakeVector 0.0 0.0 (Variables|Default|GetForce%20Z)) "None" true)
          (CallFunction|CalculateSpeed)
          (CallFunction|LaserPoint)
          (Development|PrintString (Utilities|String|Append "------------------------------------------ 
PRESS 'F11' to go fullscreen, 'Alt + P' to play-in-editor 
 
PRESS 'P' or 'ESC' to Pause & Unpause 
 
PRESS 'M' to toggle between low health (10) or high (100)  
(for ease in debug / playtest)) 
 
PRESS Z to toggle autopilot (experimental - debug) 
------------------------------------------ 
" (Utilities|String|Append "Speed : " (Utilities|String|ToString(Float) (Variables|Default|GetSpeed)) " 
Throttle : " (Utilities|String|ToString(Integer) (Variables|Default|GetThrottle)) "%" " 
Distance : " (Utilities|String|ToString(Integer) (Variables|Default|GetVeinCount)) " 
Min Throttle : " (Utilities|String|ToString(Integer) (Variables|Default|GetMinThrottle)) " 
Health : " (Utilities|String|ToString(Integer) (Variables|Default|GetHealth)) " ")) (Variables|Default|GetisDebugMode?) false "(R=1.000000,G=1.000000,B=1.000000,A=1.000000)" (Variables|Default|GetDelta%20Seconds))
          (if (>= 0 (Variables|Default|GetHealth))
            (Development|PrintString "Death" true true "(R=0.000000,G=0.660000,B=1.000000,A=1.000000)" 5.0)
            (CallFunction|GameOver)
            (goto _label Reset)))))))

(event Game|Damage|EventAnyDamage
  (params (Damage :type Float%20%28single-precision%29) (DamageType :type Damage%20Type%20Object%20Reference) (InstigatedBy :type Controller%20Object%20Reference) (DamageCauser :type Actor%20Object%20Reference))
  ;[1 0 0] Damage
  (if (<= (Variables|Default|GetShield) 0)
    (if (> (Variables|Default|GetHealth) 0)
      (Variables|Default|SetHealth (Math|Float|Truncate (- (Variables|Default|GetHealth) Damage))))
    (elif (>= Damage 5.0)
      (bind _result (Math|Integer|DecrementInt (Variables|Default|GetShield) :!label _label)
        (:%20%20
          (Variables|Default|SetShield _result)))
      (else
        (bind _output_get (Variables|Default|SetShieldDamage (+ Damage (Variables|Default|GetShieldDamage))))
        (if (>= _output_get 25.0)
          (Variables|Default|SetShieldDamage 0.0)
          (goto _label))))))

(event Input|ActionEvents|InputActionThrottleUP
  (params (Key :type Key%20Structure :default "None"))
  ;[0.1222 0.6799 1] Throttle Input to Booleans
  (:Pressed
    (Variables|Default|SetThrottleUP true))
  (:Released
    (Variables|Default|SetThrottleUP false)))

(event Input|ActionEvents|InputActionThrottleDOWN
  (params (Key :type Key%20Structure :default "None"))
  ;[0.1222 0.6799 1] Throttle Input to Booleans
  (:Pressed
    (Variables|Default|SetThrottleDOWN true))
  (:Released
    (Variables|Default|SetThrottleDOWN false)))

(event Input|ActionEvents|InputActionFire
  (params (Key :type Key%20Structure :default "None"))
  (bind _self self)
  (bind _skeletalmesh (Variables|Default|GetSkeletalMesh))
  ;[1 0.1689 0.139] Shooting
  (:Pressed
    (if (Variables|Default|GetcanShoot)
      (bind _output_get (Variables|Default|SetisShooting true))
      (if _output_get :!label _label
        (Variables|Default|SetcanShoot false)
        (Game|SpawnActorfromClass "/Game/RunnerAID/Blueprints/Bullet.Bullet_C" (Math|Transform|MakeTransform (+ (Transformation|GetWorldLocation _skeletalmesh) (Math|Vector|GetForwardVector _skeletalmesh)) "0, 0, 0" "0.700000,0.700000,0.700000") "Undefined" _self _self)
        (Utilities|FlowControl|Delay (Math|Float|SafeDivide 1.0 (Variables|Default|GetFireRate)))
        (Variables|Default|SetcanShoot true)
        (goto _label))))
  (:Released
    (Variables|Default|SetisShooting false)))

(event Input|ActionEvents|InputActionPause
  (params (Key :type Key%20Structure :default "None"))
  ;[0.08907 0.3929 1] Pause
  (:Pressed
    (bind _isa (Utilities|FlowControl|FlipFlop)
      (:A
        _)
      (:B
        _))
    (CallFunction|SetGamePause _isa)))

(event Input|AxisEvents|InputAxisRoll
  (params (AxisValue :type Float%20%28single-precision%29))
  ;[0.1853 0.3411 1] Roll, Pitch & Yaw Input to Torque
  (Variables|Default|SetXAxis AxisValue)
  (Class|PrimitiveComponent|AddTorqueinDegrees (Variables|Default|GetCollision) (Math|Vector|Lerp(Vector) "0, 0, 0" (* (* AxisValue (Variables|Default|GetAirHandling)) (Math|Vector|GetForwardVector (Variables|Default|GetCollision))) 0.1) "None" true))

(event Input|AxisEvents|InputAxisPitch
  (params (AxisValue :type Float%20%28single-precision%29))
  ;[0.1853 0.3411 1] Roll, Pitch & Yaw Input to Torque
  (Variables|Default|SetYAxis AxisValue)
  (Class|PrimitiveComponent|AddTorqueinDegrees (Variables|Default|GetCollision) (Math|Vector|Lerp(Vector) "0, 0, 0" (* (* AxisValue (Variables|Default|GetAirHandling)) (Math|Vector|GetRightVector (Variables|Default|GetCollision))) 0.1) "None" true))

(event Input|AxisEvents|InputAxisYaw
  (params (AxisValue :type Float%20%28single-precision%29))
  ;[0.1853 0.3411 1] Roll, Pitch & Yaw Input to Torque
  (Variables|Default|SetZAxis AxisValue)
  (Class|PrimitiveComponent|AddTorqueinDegrees (Variables|Default|GetCollision) (Math|Vector|Lerp(Vector) "0, 0, 0" (* (* AxisValue (Variables|Default|GetAirHandling)) (Math|Vector|GetUpVector (Variables|Default|GetCollision))) 0.1) "None" true))

(event Input|KeyboardEvents|Z
  (params (Key :type Key%20Structure :default "None"))
  ;[0.4943 0.09617 1] Debug Modes
  (:Pressed
    (Utilities|FlowControl|FlipFlop
      (:A
        (CallFunction|Autopilot))
      (:B
        (CallFunction|StopMoveAlongSpline)))))

(event Input|KeyboardEvents|M
  (params (Key :type Key%20Structure :default "None"))
  ;[1 0 0] Damage
  (:Pressed
    (Utilities|FlowControl|FlipFlop
      (:A
        (Variables|Default|SetHealth 10))
      (:B
        (Variables|Default|SetHealth 100)))))

(fn ConstructionScript)

(fn ThrottleControl
  (bind _maxthrottle (Variables|Default|GetMaxThrottle))
  (bind _minthrottle (Variables|Default|GetMinThrottle))
  (if (Variables|Default|GetThrottleUP)
    (bind _result (Math|Integer|IncrementInt (Variables|Default|GetThrottle))
      (:%20%20
        (Variables|Default|SetThrottle (Math|Integer|Clamp(Integer) _result _minthrottle _maxthrottle))
        (bind _as_game_main_mode (Variables|Default|GetAs%20Game%20Main%20Mode :!label _label)
          (:then
            (Audio|SetSoundMixClassOverride "/Game/RunnerAID/Assets/SFX/SFXShipClassMix.SFXShipClassMix" "/Game/RunnerAID/Assets/SFX/SFXShip.SFXShip" (* (Variables|/Game/RunnerAID/Blueprints/GameMainMode.GameMainMode_C|GetSFXVolume _as_game_main_mode) (+ (/ (Variables|Default|GetThrottle) (Variables|Default|GetMaxThrottle)) 0.45)) (+ (/ (Variables|Default|GetThrottle) (Variables|Default|GetMaxThrottle)) 0.45) 0.0 true)
            (Audio|PushSoundMixModifier "/Game/RunnerAID/Assets/SFX/SFXShipClassMix.SFXShipClassMix"))
          (:else))))
    (elif (Variables|Default|GetThrottleDOWN)
      (bind _result_2 (Math|Integer|DecrementInt (Variables|Default|GetThrottle))
        (:%20%20
          (Variables|Default|SetThrottle (Math|Integer|Clamp(Integer) _result_2 _minthrottle _maxthrottle))
          (goto _label))))))

(fn CalculateSpeed
  (bind _collision (Variables|Default|GetCollision))
  (bind _returnvalue (Physics|GetPhysicsLinearVelocity _collision "None"))
  (Physics|SetPhysicsLinearVelocity _collision (Math|Vector|Lerp(Vector) _returnvalue (* (Math|Vector|GetForwardVector _collision) (Math|Integer|Clamp(Integer) (* (Variables|Default|GetThrottle) 25) 0 2500)) 0.01) false "None")
  (Variables|Default|SetSpeed (Math|Vector|Distance(Vector) "0, 0, 0" (Math|Vector|Lerp(Vector) _returnvalue (* (Math|Vector|GetForwardVector _collision) (Math|Integer|Clamp(Integer) (* (Variables|Default|GetThrottle) 25) 0 2500)) 0.01))))

(fn CalcDistAlongVein
  (bind _currentveinsection (Variables|Default|GetCurrentVeinSection)
    (:then
      (bind _output_get (Variables|Default|SetDistAlongVein (/ (Class|KismetMathLibrary|DegAsin (/ (Math|Vector|Distance(Vector) (Transformation|GetWorldLocation (Variables|/Game/RunnerAID/Blueprints/VeinSection.VeinSection_C|Getstart _currentveinsection)) (Transformation|GetWorldLocation (Variables|Default|GetCollision self))) 1.2e+04)) 45.0)))
      (Development|PrintString (Utilities|String|ToString(Float) _output_get) true true "(R=0.500000,G=0.197917,B=0.433996,A=1.000000)" (Variables|Default|GetDelta%20Seconds)))
    (:else
      (Variables|Default|SetDistAlongVein 0.0)))
  (return))

(fn UpdateThrustVFX
  (Effects|Components|ParticleSystem|SetFloatParameter (Variables|Default|GetThrustVFX) "User.ThrustScale" (/ (Math|Conversions|ToFloat(Integer) (Variables|Default|GetThrottle)) 1e+02)))

(fn DamagePulseVFX
  (if (> (Variables|Default|GetPulseVariable) 1.0)
    (Variables|Default|SetPulseVariable (- (Variables|Default|GetPulseVariable) 0.05))
    (Rendering|Material|SetScalarParameterValue "/Game/RunnerAID/Assets/UI/VignetteCollection.VignetteCollection" "Damage" (Variables|Default|GetPulseVariable) :!class /Script/Engine.KismetMaterialLibrary)
    (else
      (Variables|Default|SetPulseVariable (+ (Variables|Default|GetPulseVariable) 0.05)))))