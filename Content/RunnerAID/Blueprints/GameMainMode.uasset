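; GameMainMode, apparently the runner game's main game mode, persists high score and SFX and music volume through a SaveGame_BP slot.
; It loads on BeginPlay, or creates a save if none exists, and saves on EndPlay.
; Loading applies both volumes through sound mix class overrides, pushes each mix, then writes the slot back after each one.
; Saving always builds a fresh save object from the current values.
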(event EventBeginPlay
  (CallFunction|LoadGame))

(event EventEndPlay
  (params (EndPlayReason :type EEndPlayReason%20Enum :default "Destroyed"))
  (CallFunction|SaveGame))

(fn ConstructionScript)

(fn SaveGame
  (bind _returnvalue (SaveGame|CreateSaveGameObject "/Game/RunnerAID/Blueprints/SaveGame_BP.SaveGame_BP_C"))
  (bind _output_get (Variables|Default|SetSave%20Ref _returnvalue))
  (bind _assave_game_bp (Utilities|Casting|CastToSaveGame_BP _output_get))
  (Variables|/Game/RunnerAID/Blueprints/SaveGame_BP.SaveGame_BP_C|SetHigh%20Score _assave_game_bp (Variables|Default|GetHigh%20Score))
  (Variables|/Game/RunnerAID/Blueprints/SaveGame_BP.SaveGame_BP_C|SetSFXVolume _assave_game_bp (Variables|Default|GetSFXVolume))
  (Variables|/Game/RunnerAID/Blueprints/SaveGame_BP.SaveGame_BP_C|SetMusicVolume _assave_game_bp (Variables|Default|GetMusicVolume))
  (SaveGame|SaveGametoSlot (Variables|Default|GetSave%20Ref) (Variables|Default|GetSlot%20Name)))

(fn LoadGame
  (bind _returnvalue (SaveGame|DoesSaveGameExist (Variables|Default|GetSlot%20Name)))
  (if _returnvalue
    (bind _returnvalue_2 (SaveGame|LoadGamefromSlot (Variables|Default|GetSlot%20Name)))
    (bind _output_get (Variables|Default|SetSave%20Ref _returnvalue_2))
    (bind _assave_game_bp (Utilities|Casting|CastToSaveGame_BP _output_get))
    (Variables|Default|SetHigh%20Score (Variables|/Game/RunnerAID/Blueprints/SaveGame_BP.SaveGame_BP_C|GetHigh%20Score _assave_game_bp))
    (Utilities|FlowControl|Sequence
      (:then_0
        (bind _output_get_2 (Variables|Default|SetSFXVolume (Variables|/Game/RunnerAID/Blueprints/SaveGame_BP.SaveGame_BP_C|GetSFXVolume _assave_game_bp)))
        (Audio|SetSoundMixClassOverride "/Game/RunnerAID/Assets/SFX/SFXClassMix.SFXClassMix" "/Game/RunnerAID/Assets/SFX/SFX.SFX" _output_get_2 1.0 0.2 true)
        (Audio|PushSoundMixModifier "/Game/RunnerAID/Assets/SFX/SFXClassMix.SFXClassMix"))
      (:then_1
        (bind _output_get_3 (Variables|Default|SetMusicVolume (Variables|/Game/RunnerAID/Blueprints/SaveGame_BP.SaveGame_BP_C|GetMusicVolume _assave_game_bp)))
        (Audio|SetSoundMixClassOverride "/Game/RunnerAID/Assets/SFX/MusicClassMix.MusicClassMix" "/Game/RunnerAID/Assets/SFX/Music.Music" _output_get_3 1.0 0.2 true)
        (Audio|PushSoundMixModifier "/Game/RunnerAID/Assets/SFX/MusicClassMix.MusicClassMix")))
    (SaveGame|SaveGametoSlot (Variables|Default|GetSave%20Ref) (Variables|Default|GetSlot%20Name))
    (else
      (CallFunction|SaveGame))))